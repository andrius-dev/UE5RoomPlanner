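; Inventory component that holds a list of item types and tracks which one is selected.
; On BeginPlay it spawns one actor per type at the origin with its static mesh hidden, keeps no reference to them, and selects the first type.
; SelectItemAtPosition changes the selection by bounds-checked index and returns whether it was valid, while GetSelectedItem exposes it.
; GetInteriorObjects is an empty stub.
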(event `self.ReceiveBeginPlay`
  (for _array_element (`self.ItemTypes`)
    ;[1 1 1] TODO: this will be inventory item array. they will have their thumbnails, etc.
    (bind _returnvalue (`|SpawnActorFromClass` _array_element (`KismetMathLibrary.MakeTransform` (0.0 0.0 0.0)) "AlwaysSpawn" "MultiplyWithRoot" null null))
    (`SceneComponent.SetVisibility` (`StaticMeshActor.StaticMeshComponent` _returnvalue) false false)
    (set `self.SelectedItem` (`|GetArrayItem` (`self.ItemTypes`)))))

(fn `Get Interior Objects`
  (returns (InteriorObjects :type "Array of /Game/Blueprints/BP_InventoryObject Object Reference"))
  (return))

(fn `GetSelectedItem`
  (returns (NewParam :type "/Game/Blueprints/BP_InventoryObject Class Reference"))
  (return (`self.SelectedItem`)))

(fn `SelectItemAtPosition`
  (params (Index :type Integer))
  (returns (NewParam :type Boolean))
  (bind _returnvalue (and (>= Index 0) (< Index (`KismetArrayLibrary.Array_Length` (`self.ItemTypes`)))))
  (if _returnvalue
    (set `self.SelectedItem` (`|GetArrayItem` (`self.ItemTypes`) Index)))
  (return _returnvalue))