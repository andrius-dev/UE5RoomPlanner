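; Grid component that draws a tile grid on its owning actor and converts between world locations and tile coordinates.
; On BeginPlay it caches a StaticMeshActor owner's mesh location as grid origin and adds a procedural mesh with world scale reset to one.
; CreateAndRenderGrid builds row and column lines as thin quads in one mesh section using a dynamic M_Grid material.
; LocationToTile and GetTileBounds handle tile lookups from that origin.
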(event `self.ReceiveBeginPlay`
  (`|ExecutionSequence`
    (:`then_0`
      (bind _asstatic_mesh_actor (cast `StaticMeshActor` (`self.GetOwner`)))
      (set `self.StaticMeshLocation` (`self.K2_GetComponentLocation` (`StaticMeshActor.StaticMeshComponent` _asstatic_mesh_actor))))
    (:`then_1`
      ;[1 1 1] Add grid mesh to owner
      (bind _returnvalue (`|AddComponentByClass` (`self.GetOwner`) "/Script/ProceduralMeshComponent.ProceduralMeshComponent" false (`KismetMathLibrary.Conv_VectorToTransform` (`self.RenderPositionDelta`))))
      (bind _output_get (set `self.ProceduralMesh` _returnvalue))
      (`self.CreateAndRenderGrid`)
      ;[1 1 1] Ignore parent scale
      (`self.K2_SetWorldTransform` _output_get (`KismetMathLibrary.MakeTransform` (.location (`self.K2_GetComponentToWorld` _output_get)) (.rotation (`self.K2_GetComponentToWorld` _output_get))) false false))))

(fn `CreateAndRenderGrid`
  (locals (LineMaterialInstance :type "MaterialInstanceDynamic Object Reference") (LineStart :type "Float (double-precision)") (LineEnd :type "Float (double-precision)") (LineVertices :type "Array of Vector Structure") (LineTriangles :type "Array of Integer"))
  (bind _linestart (`local.LineStart`))
  (bind _linestart_2 (`local.LineStart`))
  (bind _materialinstance (`self.CreateMaterialInstance` (`self.LineColor`) (`self.LineOpacity`)))
  (set `local.LineMaterialInstance` _materialinstance)
  (`|ExecutionSequence`
    (:`then_0`
      ;[1 1 1] Create horizontal line geometry
      (for _index (range (+ (`self.RowCount`) 1))
        (set `local.LineStart` (* _index (`self.TileSize`)))
        (set `local.LineEnd` (`self.GetGridWidth`))
        (`self.CreateLine` (`KismetMathLibrary.MakeVector` _linestart) (`KismetMathLibrary.MakeVector` _linestart (`local.LineEnd`)) (`self.LineThickness`) (`local.LineVertices`) (`local.LineTriangles`))))
    (:`then_1`
      ;[1 1 1] Create vertical line geometry
      (for _index_2 (range (+ (`self.ColumnCount`) 1))
        (set `local.LineStart` (* _index_2 (`self.TileSize`)))
        (set `local.LineEnd` (`self.GetGridHeight`))
        (`self.CreateLine` (`KismetMathLibrary.MakeVector` 0.0 _linestart_2) (`KismetMathLibrary.MakeVector` (`local.LineEnd`) _linestart_2) (`self.LineThickness`) (`local.LineVertices`) (`local.LineTriangles`))))
    (:`then_2`
      ;[1 1 1] Create line meshes
      (`ProceduralMeshComponent.CreateMeshSection_LinearColor` :`self` (`self.ProceduralMesh`) :`Vertices` (`local.LineVertices`) :`Triangles` (`local.LineTriangles`))
      (`PrimitiveComponent.SetMaterial` (`self.ProceduralMesh`) 0 (`local.LineMaterialInstance`)))))

(fn `CreateLine`
  (params (Start :type "Vector Structure") (End :type "Vector Structure") (LineThickness :type "Float (double-precision)") (OutVertices :type "Array of Vector Structure") (OutTriangles :type "Array of Integer"))
  (locals (HalfThickness :type "Float (double-precision)") (ThicknessDirection :type "Vector Structure" :default (0.0 0.0 0.0)))
  (bind _returnvalue (`KismetArrayLibrary.Array_Length` (`local.OutVertices`)))
  (`|ExecutionSequence`
    (:`then_0`
      (set `local.HalfThickness` (/ LineThickness 2.0))
      (set `local.ThicknessDirection` (`KismetMathLibrary.Cross_VectorVector` (`KismetMathLibrary.Normal` (- (`local.End`) (`local.Start`))) (0.0 0.0 1.0))))
    (:`then_1`
      (`KismetArrayLibrary.Array_Append` (`local.OutTriangles`) (`|MakeArray` (+ _returnvalue 2) (+ _returnvalue 1) (+ _returnvalue 0) (+ _returnvalue 2) (+ _returnvalue 3) (+ _returnvalue 1)))
      (`KismetArrayLibrary.Array_Append` (`local.OutVertices`) (`|MakeArray` (+ (`local.Start`) (* (`local.ThicknessDirection`) (`local.HalfThickness`))) (+ (`local.End`) (* (`local.ThicknessDirection`) (`local.HalfThickness`))) (- (`local.Start`) (* (`local.ThicknessDirection`) (`local.HalfThickness`))) (- (`local.End`) (* (`local.ThicknessDirection`) (`local.HalfThickness`))))))))

(fn `CreateMaterialInstance`
  (params (Color :type "LinearColor Structure") (Opacity :type "Float (double-precision)"))
  (returns (MaterialInstance :type "MaterialInstanceDynamic Object Reference"))
  (bind _returnvalue (`KismetMaterialLibrary.CreateDynamicMaterialInstance` "/Game/InteriorData/M_Grid.M_Grid"))
  (`MaterialInstanceDynamic.SetVectorParameterValue` _returnvalue "Color" Color)
  (`MaterialInstanceDynamic.SetScalarParameterValue` _returnvalue "None" Opacity)
  (return _returnvalue))

(fn `GetGridHeight`
  (returns (Width :type "Float (double-precision)"))
  (return (* (`self.TileSize`) (`self.RowCount`))))

(fn `GetGridWidth`
  (returns (Width :type "Float (double-precision)"))
  (return (* (`self.TileSize`) (`self.ColumnCount`))))

(fn `GetTileBounds`
  (params (Row :type Integer) (Column :type Integer) (CenterLocation :type Boolean))
  (returns (WorldLocation :type "Vector Structure"))
  (bind (_staticmeshlocation_x _staticmeshlocation_y) (`KismetMathLibrary.BreakVector` (`self.StaticMeshLocation`)))
  (bind _staticmeshlocation_x_2 (`KismetMathLibrary.BreakVector` (`self.StaticMeshLocation`)))
  (bind _returnvalue (/ (`self.TileSize`) 2.0))
  (bind _returnvalue_2 (`KismetMathLibrary.MakeVector` (+ (* (`local.Row`) (`self.TileSize`)) _staticmeshlocation_x_2) (+ (* (`local.Column`) (`self.TileSize`)) _staticmeshlocation_y)))
  (if (`local.CenterLocation`)
    (return (+ _returnvalue_2 (`KismetMathLibrary.MakeVector` _returnvalue _returnvalue)))
    (else
      (return _returnvalue_2))))

(fn `LocationToTile`
  (params (WorldLocation :type "Vector Structure"))
  (returns (IsValid :type Boolean) (Row :type Integer) (Column :type Integer))
  (bind (_staticmeshlocation_x _staticmeshlocation_y) (`KismetMathLibrary.BreakVector` (`self.StaticMeshLocation`)))
  (bind _staticmeshlocation_x_2 (`KismetMathLibrary.BreakVector` (`self.StaticMeshLocation`)))
  (return true (`KismetMathLibrary.FFloor` (* (`self.RowCount`) (/ (- WorldLocation_X _staticmeshlocation_x_2) (`self.GetGridHeight`)))) (`KismetMathLibrary.FFloor` (* (`self.ColumnCount`) (/ (- WorldLocation_Y _staticmeshlocation_y) (`self.GetGridWidth`))))))