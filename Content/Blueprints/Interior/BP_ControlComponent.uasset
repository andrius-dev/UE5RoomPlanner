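; BP_ControlComponent is an actor component that adds a clickable arrow mesh to its owning actor, apparently as an interior control.
; On BeginPlay it creates a static mesh component on the owner at runtime, offset along negative Y and raised by configurable center and floor distances.
; It assigns the arrow mesh and binds its click event, which currently only prints a debug message.
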(event `self.ReceiveBeginPlay`
  (bind _returnvalue (`|AddComponentByClass` (`self.GetOwner`) "/Script/Engine.StaticMeshComponent" false (`KismetMathLibrary.MakeTransform` (`KismetMathLibrary.MakeVector` 0.0 (* (`self.DistanceFromCenter`) -1.0) (`self.DistanceFromFloor`)))))
  (`StaticMeshComponent.SetStaticMesh` _returnvalue (`self.ArrowMesh`))
  (add `PrimitiveComponent.OnClicked` _returnvalue (delegate `OnClicked_Event`)))

(event `OnClicked_Event`
  (params (TouchedComponent :type "PrimitiveComponent Object Reference") (ButtonPressed :type "Key Structure" :default "None"))
  (`KismetSystemLibrary.PrintString` "Arrow clicked!"))