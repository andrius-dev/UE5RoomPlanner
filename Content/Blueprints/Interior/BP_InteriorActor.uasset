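; Interior item actor that takes its static mesh from its InItemData.
; On BeginPlay it applies that mesh to its StaticMeshComponent and prints a debug message if the assignment fails.
; AsStaticMeshActor returns the actor itself and GetData exposes the item data to other code.
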(event `self.ReceiveBeginPlay`
  (bind _returnvalue (`StaticMeshComponent.SetStaticMesh` (`self.StaticMeshComponent`) (`.StaticMesh_5_821C9AA9C2C64218892A07426DEE515C` (break `/Game/Blueprints/Interior/F_InteriorItemData` (`self.InItemData`)))))
  (if (not _returnvalue)
    (`KismetSystemLibrary.PrintString` (`KismetStringLibrary.BuildString_Object` "Failed to set static mesh: "))))

(fn `As Static Mesh Actor`
  (returns (StaticMesh :type "StaticMeshActor Object Reference"))
  (return self))

(fn `GetData`
  (returns (ItemData :type "/Game/Blueprints/Interior/F_InteriorItemData Structure"))
  (return (`self.InItemData`)))

(fn `UserConstructionScript`)