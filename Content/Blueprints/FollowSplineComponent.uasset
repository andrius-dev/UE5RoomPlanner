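; Actor component that moves its owner along a BP_TargetSpline, optionally picking the spline nearest its forward aim point on BeginPlay.
; Each tick it records distance and percentage along the spline, then projects a point ahead of the owner onto the spline as the destination.
; The owner advances on local X at a framerate-independent speed and snaps its rotation toward that destination, giving look-ahead path following.
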(event `self.ReceiveBeginPlay`
  ;[1 1 1] AutoFind closest spline on Play
  (if (`self.Auto Find Spline`)
    (bind _outactors (`GameplayStatics.GetAllActorsOfClass` "/Game/Blueprints/BP_TargetSpline.BP_TargetSpline_C"))
    (bind _asbp_target_spline (cast `/Game/Blueprints/BP_TargetSpline` (`.ReturnValue` (`GameplayStatics.FindNearestActor` (`self.Get Forward Aim Location`) _outactors))))
    (set `self.Target Spline` _asbp_target_spline)))

(event `self.ReceiveTick`
  (params (DeltaSeconds :type "Float (single-precision)"))
  (`self.Get Current Distance On Spline`)
  (`self.UpdateDestination`)
  (`self.ProceedToDestination` DeltaSeconds))

(fn `Get Current Distance On Spline`
  (bind _splinepath (`/Game/Blueprints/BP_TargetSpline.SplinePath` (`self.Target Spline`)))
  (bind _output_get (set `self.DistanceAlongSpline` (`SplineComponent.GetDistanceAlongSplineAtSplineInputKey` _splinepath (`SplineComponent.FindInputKeyClosestToWorldLocation` _splinepath (`Actor.K2_GetActorLocation` (`self.GetOwner`))))))
  (set `self.PercentageAlongSpline` (* (/ _output_get (`SplineComponent.GetSplineLength` _splinepath)) 100.0)))

(fn `Get Forward Aim Location`
  (returns (`Front Location` :type "Vector Structure"))
  (bind _returnvalue (`self.GetOwner`))
  (return (+ (`Actor.K2_GetActorLocation` _returnvalue) (* (`Actor.GetActorForwardVector` _returnvalue) (`self.ForwardAimDistance`)))))

(fn `ProceedToDestination`
  (params (DeltaTime :type "Float (double-precision)"))
  (locals (TimeSinceLastUpdate :type "Float (double-precision)"))
  (bind _returnvalue (`self.GetOwner`))
  (bind _rootcomponent (`Actor.RootComponent` _returnvalue))
  (set `local.TimeSinceLastUpdate` DeltaTime)
  (`Actor.K2_AddActorLocalOffset` _returnvalue (`KismetMathLibrary.MakeVector` (* (* (`self.Speed`) (`self.MaxSpeed cm/s`)) (`local.TimeSinceLastUpdate`))) false false)
  (`SceneComponent.K2_SetWorldRotation` _rootcomponent (`KismetMathLibrary.FindLookAtRotation` (`SceneComponent.K2_GetComponentLocation` _rootcomponent) (`self.Destination`)) false false))

(fn `UpdateDebug`
  (`KismetSystemLibrary.DrawDebugSphere` (`self.Destination`) 10.0 12 (struct :`R` 1.0 :`A` 1.0))
  (`KismetSystemLibrary.DrawDebugSphere` (`self.Get Forward Aim Location`) 10.0 12 (struct :`G` 0.014911 :`B` 1.0 :`A` 1.0)))

(fn `UpdateDestination`
  (set `self.Destination` (`SplineComponent.FindLocationClosestToWorldLocation` (`/Game/Blueprints/BP_TargetSpline.SplinePath` (`self.Target Spline`)) (`self.Get Forward Aim Location`) "World")))