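; BP_InteriorEditComponent handles placing and selecting interior items for the player's BP_EditorPawn.
; It binds to the pawn's palette, click, creation and floor-hover events, turning palette picks into actor creation calls.
; InteriorItem gameplay tags, set through BI_InteriorActorInterface, track state: a Placing actor follows the hovered floor location.
; Clicking an interior actor switches it to Editing and broadcasts its data to start editing.
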(event `self.ReceiveBeginPlay`
  (bind _asbp_editor_pawn (cast `/Game/Blueprints/Player/BP_EditorPawn` (`self.GetOwner`))
    (:`then`
      (bind _output_get (set `self.OwnerPawn` _asbp_editor_pawn))
      (add `/Game/Blueprints/Player/BP_EditorPawn.OnPaletteItemSelected` _output_get (`|CreateDelegate` :!event `EventPaletteItemSelected`))
      (add `/Game/Blueprints/Player/BP_EditorPawn.OnActorClicked` (`self.OwnerPawn`) (`|CreateDelegate` :!event `EventActorClicked`))
      (add `/Game/Blueprints/Player/BP_EditorPawn.OnInteriorActorCreated` (`self.OwnerPawn`) (`|CreateDelegate` :!event `EventInteriorActorCreated`))
      (add `/Game/Blueprints/Player/BP_EditorPawn.OnMouseHoverOverFloor` (`self.OwnerPawn`) (`|CreateDelegate` :!event `EventPlayerHoverMouseOverFloor`)))
    (:`CastFailed`
      (`KismetSystemLibrary.PrintString` "BP_InteriorActor: Owner should be editor!")
      (`KismetSystemLibrary.QuitGame` null "Quit"))))

(event `EventPaletteItemSelected`
  (params (ItemData :type "/Game/UI/Data/F_PaletteItemData Structure"))
  (bind _outdata (`/Game/Blueprints/BP_EditorUtilities.PaletteDataToInteriorActorData` ItemData))
  (`self.OnCreateInteriorActor` _outdata))

(event `EventPlayerHoverMouseOverFloor`
  (params (WorldLocation :type "Vector Structure"))
  (bind _tags (message `/Game/Blueprints/Interior/BI_InteriorActorInterface.GetGameplayTags` (`self.InteriorActor`)))
  (if (`BlueprintGameplayTagLibrary.HasTag` _tags (struct :`TagName` "InteriorItem.Placing") true)
    (`Actor.K2_SetActorLocation` (`self.InteriorActor`) WorldLocation false false)))

(event `EventActorClicked`
  (params (Actor :type "Actor Object Reference") (ClickLocation :type "Vector Structure"))
  (if (`KismetSystemLibrary.DoesImplementInterface` Actor "/Game/Blueprints/Interior/BI_InteriorActorInterface.BI_InteriorActorInterface_C")
    ;[1 1 1] Clear previously selected actor's tags
    (message `/Game/Blueprints/Interior/BI_InteriorActorInterface.RemoveGameplayTag` (`self.InteriorActor`) (struct :`TagName` "InteriorItem.Editing"))
    (bind _output_get (set `self.InteriorActor` Actor))
    (bind _itemdata (message `/Game/Blueprints/Interior/BI_InteriorActorInterface.GetData` _output_get))
    (`self.OnEditRoomActorStarted` _itemdata)
    (message `/Game/Blueprints/Interior/BI_InteriorActorInterface.RemoveGameplayTag` (`self.InteriorActor`) (struct :`TagName` "InteriorItem.Placing"))
    (message `/Game/Blueprints/Interior/BI_InteriorActorInterface.AddGameplayTag` (`self.InteriorActor`) (struct :`TagName` "InteriorItem.Editing"))))

(event `EventInteriorActorCreated`
  (params (InteriorActor :type "Actor Object Reference"))
  (if (`KismetSystemLibrary.DoesImplementInterface` InteriorActor "/Game/Blueprints/Interior/BI_InteriorActorInterface.BI_InteriorActorInterface_C")
    (bind _output_get (set `self.InteriorActor` InteriorActor))
    (message `/Game/Blueprints/Interior/BI_InteriorActorInterface.AddGameplayTag` _output_get (struct :`TagName` "InteriorItem.Placing"))
    (else
      (`KismetSystemLibrary.PrintString` "Created actor doesn't implement InteriorActorInterface!"))))