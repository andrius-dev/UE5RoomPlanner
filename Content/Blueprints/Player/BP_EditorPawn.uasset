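; Player pawn for an interior editor that creates the editor screen and turns mouse input into editing events.
; Cursor traces broadcast clicked actors and, every tick, hovered floor points with their tile locations from the floor's grid interface.
; Palette selections are rebroadcast, while BP_InteriorEditComponent events spawn interior actors from data and toggle the edit panel.
; Camera zoom input is a stub with a zero movement vector.
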(event `self.ReceiveBeginPlay`
  (`|ExecutionSequence`
    (:`then_1`
      (bind _returnvalue (`|CreateWidget` "/Game/UI/WB_EditorScreen.WB_EditorScreen_C"))
      (`UserWidget.AddToViewport` _returnvalue 0)
      (bind _output_get (set `self.EditorScreen` _returnvalue))
      (add `/Game/UI/WB_PalettePanel.OnItemSelected` (`/Game/UI/WB_EditorScreen.WB_PalettePanel` _output_get) (delegate `ItemSelected`)))))

(event `ItemSelected`
  (params (ItemObject :type "/Game/UI/Data/F_PaletteItemData Structure"))
  (`self.OnPaletteItemSelected` ItemObject))

(event `EnhancedInput|/Game/Input/IA_Select`
  (params (ActionValue :type Boolean) (ElapsedSeconds :type "Float (double-precision)") (TriggeredSeconds :type "Float (double-precision)") (InputAction :type "InputAction Object Reference" :default "/Game/Input/IA_Select.IA_Select"))
  (:`Triggered`
    (bind (_outhit _isvalid) (`self.GetMouseHoveredActor`))
    (if _isvalid
      (bind (_bblockinghit _binitialoverlap _time _distance _location _impactpoint _normal _impactnormal _physmat _hitactor) (`GameplayStatics.BreakHitResult` _outhit))
      (`self.OnActorClicked` _hitactor _location))))

(event `EnhancedInput|/Game/Input/IA_ZoomCamera`
  (params (ActionValue :type "Float (double-precision)") (ElapsedSeconds :type "Float (double-precision)") (TriggeredSeconds :type "Float (double-precision)") (InputAction :type "InputAction Object Reference" :default "/Game/Input/IA_ZoomCamera.IA_ZoomCamera"))
  (:`Triggered`
    (`self.AddMovementInput` (0.0 0.0 0.0))))

(event `self.ReceiveTick`
  (params (DeltaSeconds :type "Float (single-precision)"))
  (bind (_isvalid _clicklocation _tilelocation) (`self.GetMouseHoveredFloorInfo`))
  (if _isvalid
    (`self.OnMouseHoverOverFloor` _clicklocation _tilelocation)))

(event `self.BP_InteriorEditComponent.OnCreateInteriorActor`
  (params (ActorData :type "/Game/Blueprints/Interior/F_InteriorItemData Structure"))
  (bind _interioractor (`self.SpawnInteriorActorFromData` ActorData))
  (`self.OnInteriorActorCreated` _interioractor))

(event `self.BP_InteriorEditComponent.OnEditRoomActorStarted`
  (params (ActorData :type "/Game/Blueprints/Interior/F_InteriorItemData Structure"))
  (`/Game/UI/WB_EditorScreen.OnShowEditPanel` (`self.EditorScreen`) ActorData))

(event `self.BP_InteriorEditComponent.OnEditRoomActorFinished`
  (`/Game/UI/WB_EditorScreen.OnHideEditPanel` (`self.EditorScreen`)))

(fn `GetGameplayTags`
  (returns (Tags :type "GameplayTagContainer Structure"))
  (return (`self.GameplayTags`)))

(fn `GetMouseHoveredActor`
  (returns (OutHit :type "HitResult Structure") (IsValid :type Boolean))
  (bind (_worldlocation _worlddirection) (`PlayerController.DeprojectMousePositionToWorld` (`self.GetLocalViewingPlayerController`)))
  (bind (_outhit _returnvalue) (`KismetSystemLibrary.LineTraceSingleForObjects` _worldlocation (+ _worldlocation (* _worlddirection (`self.MaxDistanceToClickedActor`))) (`|MakeArray` "ObjectTypeQuery3" "ObjectTypeQuery2" :!type "EObjectTypeQuery Enum")))
  (return _outhit _returnvalue))

(fn `GetMouseHoveredFloorInfo`
  (returns (IsValid :type Boolean) (ClickLocation :type "Vector Structure") (TileLocation :type "Vector Structure"))
  (bind (_worldlocation _worlddirection) (`PlayerController.DeprojectMousePositionToWorld` (`self.GetLocalViewingPlayerController`)))
  (bind (_outhit _returnvalue) (`KismetSystemLibrary.LineTraceSingleForObjects` _worldlocation (+ _worldlocation (* _worlddirection (`self.MaxDistanceToClickedActor`))) (`|MakeArray` "ObjectTypeQuery1" "ObjectTypeQuery2" "ObjectTypeQuery3" "ObjectTypeQuery6" "ObjectTypeQuery1" :!type "EObjectTypeQuery Enum")))
  (if _returnvalue
    (bind (_bblockinghit _binitialoverlap _time _distance _location _impactpoint _normal _impactnormal _physmat _hitactor) (`GameplayStatics.BreakHitResult` _outhit))
    (if (`KismetSystemLibrary.DoesImplementInterface` _hitactor "/Game/Blueprints/Interior/BI_FloorInterface.BI_FloorInterface_C")
      (bind _gridcomponent (message `/Game/Blueprints/Interior/BI_FloorInterface.GetGridComponent` _hitactor))
      (bind (_isvalid _row _column) (`/Game/Blueprints/Interior/BP_GridComponent.LocationToTile` _gridcomponent _location))
      (if _isvalid
        (bind (_isvalid_2 _worldlocation_2) (`/Game/Blueprints/Interior/BP_GridComponent.GetTileBounds` _gridcomponent _row _column true))
        (return true _location _worldlocation_2)))
    (else
      (return false (0.0 0.0 0.0) (0.0 0.0 0.0)))))

(fn `SpawnInteriorActorFromData`
  (params (Data :type "/Game/Blueprints/Interior/F_InteriorItemData Structure"))
  (returns (InteriorActor :type "/Game/Blueprints/Interior/BP_InteriorActor Object Reference"))
  (bind _returnvalue (`|SpawnActorFromClass` "/Game/Blueprints/Interior/BP_InteriorActor.BP_InteriorActor_C" (`.WorldTransform_11_F066552B213D4F41B76C50C33F11B003` (break `/Game/Blueprints/Interior/F_InteriorItemData` Data)) "AlwaysSpawn" "MultiplyWithRoot" self Data null))
  (return _returnvalue))

(fn `UserConstructionScript`)