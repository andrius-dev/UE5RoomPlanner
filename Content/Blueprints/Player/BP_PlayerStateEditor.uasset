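; BP_PlayerStateEditor is a player-side Blueprint that holds the current edit state object for an editor mode.
; On BeginPlay it constructs an object from InitialEditStateClass and sets it as the edit state.
; SetEditState stores the new state, prints it on screen for debugging and fires the OnEditStateChanged dispatcher.
; GetEditState exposes the current state to other code.
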(event `self.ReceiveBeginPlay`
  (bind _returnvalue (`|GenericCreateObject` (`self.InitialEditStateClass`)))
  (`self.SetEditState` _returnvalue))

(fn `GetEditState`
  (returns (NewParam :type "/Game/Blueprints/EditState/BP_BaseEditState Object Reference"))
  (return (`self.EditState`)))

(fn `SetEditState`
  (params (NewEditState :type "/Game/Blueprints/EditState/BP_BaseEditState Object Reference"))
  (bind _output_get (set `self.EditState` NewEditState))
  (`KismetSystemLibrary.PrintString` (`KismetStringLibrary.BuildString_Object` "Setting state to: " "" _output_get) true true (struct :`R` 1.0 :`G` 0.015278 :`A` 1.0) 30.0)
  (`self.OnEditStateChanged` NewEditState)
  (return))

(fn `UserConstructionScript`)