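; Player pawn for an interior editor, where palette items are spawned, placed on the floor and selected for editing.
; It creates the editor screen and drives edit-state objects (Selecting, Placing, Editing) stored on the player state, whose changes show or hide the edit panel.
; Mouse-ray object traces handle click selection through an interface and move the placed item across floor-tagged surfaces each Tick.
; Camera zoom is a zero-vector stub.
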(event `self.ReceiveBeginPlay`
  (`|ExecutionSequence`
    (:`then_0`
      (bind _asbp_player_state_editor (cast `/Game/Blueprints/Player/BP_PlayerStateEditor` (`GameplayStatics.GetPlayerState` 0)))
      (set `self.State` _asbp_player_state_editor))
    (:`then_1`
      (bind _returnvalue (`|CreateWidget` "/Game/UI/WB_EditorScreen.WB_EditorScreen_C"))
      (`UserWidget.AddToViewport` _returnvalue 0)
      (bind _output_get (set `self.EditorScreen` _returnvalue))
      (add `/Game/UI/WB_PalettePanel.OnItemSelected` (`/Game/UI/WB_EditorScreen.WB_PalettePanel` _output_get) (`|CreateDelegate` :!event `OnPaletteItemSelected`)))
    (:`then_2`
      (add `/Game/Blueprints/Player/BP_PlayerStateEditor.OnEditStateChanged` (`self.State`) (delegate `OnEditStateChanged`)))))

(event `OnPaletteItemSelected`
  (params (PaletteDataObject :type "/Game/UI/Data/F_PaletteItem Structure"))
  (bind _interioractor (`self.SpawnInteriorObjectFromData` PaletteDataObject))
  (bind _returnvalue (`|GenericCreateObject` "/Game/Blueprints/EditState/BP_EditStatePlacingObject.BP_EditStatePlacingObject_C" _interioractor))
  (`/Game/Blueprints/Player/BP_PlayerStateEditor.SetEditState` (`self.State`) _returnvalue))

(event `OnEditStateChanged`
  (params (NewEditState :type "/Game/Blueprints/EditState/BP_BaseEditState Object Reference"))
  (`KismetSystemLibrary.PrintString` (`KismetStringLibrary.BuildString_Object` "Edit state changed:" "" NewEditState) true true (struct :`G` 0.66 :`B` 1.0 :`A` 1.0) 30.0)
  (bind _editstate (`/Game/Blueprints/EditState/BI_EditStateInterface.GetStateEnum` NewEditState))
  (switch `/Game/Blueprints/EditState/E_EditState` _editstate
    (:`NewEnumerator0`
      (`/Game/UI/WB_EditorScreen.OnHideEditPanel` (`self.EditorScreen`) :!label _label))
    (:`NewEnumerator1`
      (goto _label))
    (:`NewEnumerator2`
      (bind _asbp_edit_state_editing_item (cast `/Game/Blueprints/EditState/BP_EditStateEditingItem` NewEditState))
      (`/Game/UI/WB_EditorScreen.OnShowEditPanel` (`self.EditorScreen`) (`/Game/Blueprints/EditState/BP_EditStateEditingItem.EditData` _asbp_edit_state_editing_item)))))

(event `EnhancedInput|/Game/Input/IA_Select`
  (params (ActionValue :type Boolean) (ElapsedSeconds :type "Float (double-precision)") (TriggeredSeconds :type "Float (double-precision)") (InputAction :type "InputAction Object Reference" :default "/Game/Input/IA_Select.IA_Select"))
  (:`Triggered`
    (bind (_outhit _isvalid) (`self.GetMouseHoveredActor`))
    (if _isvalid
      (bind (_bblockinghit _binitialoverlap _time _distance _location _impactpoint _normal _impactnormal _physmat _hitactor _hitcomponent) (`GameplayStatics.BreakHitResult` _outhit))
      (`self.HandleSelectButtonClicked` _hitactor _location))))

(event `EnhancedInput|/Game/Input/IA_ZoomCamera`
  (params (ActionValue :type "Float (double-precision)") (ElapsedSeconds :type "Float (double-precision)") (TriggeredSeconds :type "Float (double-precision)") (InputAction :type "InputAction Object Reference" :default "/Game/Input/IA_ZoomCamera.IA_ZoomCamera"))
  (:`Triggered`
    (`self.AddMovementInput` (0.0 0.0 0.0))))

(event `self.ReceiveTick`
  (params (DeltaSeconds :type "Float (single-precision)"))
  (bind _newparam (`/Game/Blueprints/Player/BP_PlayerStateEditor.GetEditState` (`self.State`)))
  (if (`GameplayStatics.ObjectIsA` _newparam "/Game/Blueprints/EditState/BP_EditStatePlacingObject.BP_EditStatePlacingObject_C")
    (bind _asbp_edit_state_placing_object (cast `/Game/Blueprints/EditState/BP_EditStatePlacingObject` _newparam))
    (bind _location (`self.Get Mouse Location on Floor`))
    (`self.K2_SetActorLocation` (`/Game/Blueprints/EditState/BP_EditStatePlacingObject.InteriorActor` _asbp_edit_state_placing_object) _location false false)))

(fn `Get Mouse Location on Floor`
  (returns (Location :type "Vector Structure") (IsValid :type Boolean))
  (bind (_worldlocation _worlddirection) (`PlayerController.DeprojectMousePositionToWorld` (`self.GetLocalViewingPlayerController`)))
  (bind (_outhit _returnvalue) (`KismetSystemLibrary.LineTraceSingleForObjects` _worldlocation (+ _worldlocation (* _worlddirection (`self.MaxDistanceToClickedActor`))) (`|MakeArray` "ObjectTypeQuery1" :!type "EObjectTypeQuery Enum")))
  (if _returnvalue
    (bind (_bblockinghit _binitialoverlap _time _distance _location _impactpoint _normal _impactnormal _physmat _hitactor) (`GameplayStatics.BreakHitResult` _outhit))
    (if (`self.ActorHasTag` _hitactor (`self.TagFloor`))
      (return _location true))
    (else
      (return (0.0 0.0 0.0) false))))

(fn `GetGameplayTags`
  (returns (Tags :type "GameplayTagContainer Structure"))
  (return (`self.GameplayTags`)))

(fn `GetMouseHoveredActor`
  (returns (OutHit :type "HitResult Structure") (IsValid :type Boolean))
  (bind (_worldlocation _worlddirection) (`PlayerController.DeprojectMousePositionToWorld` (`self.GetLocalViewingPlayerController`)))
  (bind (_outhit _returnvalue) (`KismetSystemLibrary.LineTraceSingleForObjects` _worldlocation (+ _worldlocation (* _worlddirection (`self.MaxDistanceToClickedActor`))) (`|MakeArray` "ObjectTypeQuery3" "ObjectTypeQuery2" :!type "EObjectTypeQuery Enum")))
  (return _outhit _returnvalue))

(fn `HandleSelectButtonClicked`
  (params (SelectedActor :type "Actor Object Reference") (ClickLocation :type "Vector Structure (by ref)"))
  (locals (TempSelectedActor :type "Actor Object Reference"))
  (bind _tempselectedactor (`local.TempSelectedActor`))
  (bind _output_get (set `local.TempSelectedActor` SelectedActor))
  (if (`KismetSystemLibrary.DoesImplementInterface` _output_get "/Game/Blueprints/Interior/BI_InteriorActorInterface.BI_InteriorActorInterface_C")
    (bind _itemdata (message `/Game/Blueprints/Interior/BI_InteriorActorInterface.GetData` (`local.TempSelectedActor`)))
    (bind _returnvalue (`|GenericCreateObject` "/Game/Blueprints/EditState/BP_EditStateEditingItem.BP_EditStateEditingItem_C" _itemdata))
    (`/Game/Blueprints/Player/BP_PlayerStateEditor.SetEditState` (`self.State`) _returnvalue)
    (else
      (bind _newparam (`/Game/Blueprints/Player/BP_PlayerStateEditor.GetEditState` (`self.State`)))
      (bind _editstate (`/Game/Blueprints/EditState/BI_EditStateInterface.GetStateEnum` _newparam))
      (switch `/Game/Blueprints/EditState/E_EditState` _editstate
        (:`NewEnumerator0`
          (if (`KismetSystemLibrary.DoesImplementInterface` _tempselectedactor "/Game/Blueprints/Interior/BI_InteriorActorInterface.BI_InteriorActorInterface_C")
            (bind _itemdata_2 (message `/Game/Blueprints/Interior/BI_InteriorActorInterface.GetData` _tempselectedactor))
            (bind _returnvalue_2 (`|GenericCreateObject` "/Game/Blueprints/EditState/BP_EditStateEditingItem.BP_EditStateEditingItem_C" _itemdata_2))
            (`/Game/Blueprints/Player/BP_PlayerStateEditor.SetEditState` (`self.State`) _returnvalue_2)
            (return)))
        (:`NewEnumerator1`
          (bind _asbp_edit_state_placing_object (cast `/Game/Blueprints/EditState/BP_EditStatePlacingObject` _newparam))
          (if (`self.ActorHasTag` (`local.TempSelectedActor`) "Floor")
            (bind _itemdata_3 (`/Game/Blueprints/Interior/BI_InteriorActorInterface.GetData` (`/Game/Blueprints/EditState/BP_EditStatePlacingObject.InteriorActor` _asbp_edit_state_placing_object)))
            (bind _returnvalue_3 (`|GenericCreateObject` "/Game/Blueprints/EditState/BP_EditStateEditingItem.BP_EditStateEditingItem_C" _itemdata_3))
            (`/Game/Blueprints/Player/BP_PlayerStateEditor.SetEditState` (`self.State`) _returnvalue_3)
            (return)))
        (:`NewEnumerator2`
          (if (`self.ActorHasTag` (`local.TempSelectedActor`) "Floor")
            _))))))

(fn `PaletteItemToInteriorActor`
  (params (InData :type "/Game/UI/Data/F_PaletteItem Structure"))
  (returns (OutData :type "/Game/Blueprints/Interior/F_InteriorItemData Structure"))
  (bind (_title _image _staticmesh) (break `/Game/UI/Data/F_PaletteItem` InData))
  (return (make `/Game/Blueprints/Interior/F_InteriorItemData` _title _staticmesh (make `Color` 0) (`KismetMathLibrary.MakeTransform` (0.0 0.0 0.0)))))

(fn `SpawnInteriorObjectFromData`
  (params (Data :type "/Game/UI/Data/F_PaletteItem Structure"))
  (returns (InteriorActor :type "/Game/Blueprints/Interior/BP_InteriorActor Object Reference"))
  (bind _outdata (`self.PaletteItemToInteriorActor` Data))
  (bind _returnvalue (`|SpawnActorFromClass` "/Game/Blueprints/Interior/BP_InteriorActor.BP_InteriorActor_C" (`.WorldTransform_11_F066552B213D4F41B76C50C33F11B003` (break `/Game/Blueprints/Interior/F_InteriorItemData` _outdata)) "AlwaysSpawn" "MultiplyWithRoot" self _outdata null))
  (return _returnvalue))

(fn `UserConstructionScript`)