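; Editor pawn component that handles placing, selecting, moving, recoloring and deleting interior items in a room editor.
; On BeginPlay it binds to BP_EditorPawn events and relays palette picks, edit start and edit finish through its own dispatchers.
; Gameplay tags on the current EditableItem track placing, editing and moving states, deciding whether it follows floor hover, with optional grid snapping.
; Color changes apply through a dynamic material instance.
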(event `self.ReceiveBeginPlay`
  ;[1 1 1] Binding to Editor Pawn events
  (bind _asbp_editor_pawn (cast `/Game/Blueprints/Player/BP_EditorPawn` (`self.GetOwner`))
    (:`then`
      (bind _output_get (set `self.OwnerPawn` _asbp_editor_pawn))
      (add `/Game/Blueprints/Player/BP_EditorPawn.OnPaletteItemSelected` _output_get (`|CreateDelegate` :!event `EventPaletteItemSelected`))
      (add `/Game/Blueprints/Player/BP_EditorPawn.OnActorClicked` (`self.OwnerPawn`) (`|CreateDelegate` :!event `EventActorClicked`))
      (add `/Game/Blueprints/Player/BP_EditorPawn.OnInteriorActorCreated` (`self.OwnerPawn`) (`|CreateDelegate` :!event `EventInteriorActorCreated`))
      (add `/Game/Blueprints/Player/BP_EditorPawn.OnMouseHoverOverFloor` (`self.OwnerPawn`) (`|CreateDelegate` :!event `EventHoverMouseOverFloor`))
      (add `/Game/Blueprints/Player/BP_EditorPawn.OnMoveEditableItem` (`self.OwnerPawn`) (`|CreateDelegate` :!event `EventEditableItemMove`))
      (add `/Game/Blueprints/Player/BP_EditorPawn.OnDeleteEditableItem` (`self.OwnerPawn`) (`|CreateDelegate` :!event `EventEditableItemDelete`))
      (add `/Game/Blueprints/Player/BP_EditorPawn.OnItemColorSelected` (`self.OwnerPawn`) (`|CreateDelegate` :!event `EventItemColorSelected`)))
    (:`CastFailed`
      (`KismetSystemLibrary.PrintString` "BP_InteriorActor: Owner should be editor!")
      (`KismetSystemLibrary.QuitGame` null "Quit"))))

(event `EventHoverMouseOverFloor`
  (params (WorldLocation :type "Vector Structure") (TileLocation :type "Vector Structure"))
  (bind _editableitem (`self.EditableItem`))
  ;[1 1 1] Move interior item if it has movable tags
  (if (`KismetSystemLibrary.DoesImplementInterface` _editableitem "/Game/Blueprints/Interior/BI_InteriorActorInterface.BI_InteriorActorInterface_C")
    (bind _tags (message `/Game/Blueprints/Interior/BI_InteriorActorInterface.GetGameplayTags` _editableitem))
    (if (`BlueprintGameplayTagLibrary.HasAnyTags` _tags (`self.MoveTags`) true)
      (if (`self.IsSnapToGridEnabled`)
        (`Actor.K2_SetActorLocation` (`self.EditableItem`) TileLocation false false)
        (else
          (`Actor.K2_SetActorLocation` (`self.EditableItem`) WorldLocation false false))))))

(event `EventActorClicked`
  (params (Actor :type "Actor Object Reference") (ClickLocation :type "Vector Structure"))
  (if (`KismetSystemLibrary.DoesImplementInterface` Actor "/Game/Blueprints/Interior/BI_InteriorActorInterface.BI_InteriorActorInterface_C")
    (`|ExecutionSequence`
      (:`then_0`
        ;[1 1 1] Clear previously selected actor's tags
        (message `/Game/Blueprints/Interior/BI_InteriorActorInterface.RemoveGameplayTag` (`self.EditableItem`) (struct :`TagName` "InteriorItem.Editing"))
        (set `self.EditableItem` Actor))
      (:`then_1`
        ;[1 1 1] Setup item tags so it's not moving
        (bind _itemdata (message `/Game/Blueprints/Interior/BI_InteriorActorInterface.GetData` (`self.EditableItem`)))
        (`self.OnEditRoomActorStarted` _itemdata)
        (message `/Game/Blueprints/Interior/BI_InteriorActorInterface.RemoveGameplayTag` (`self.EditableItem`) (struct :`TagName` "InteriorItem.Placing"))
        (message `/Game/Blueprints/Interior/BI_InteriorActorInterface.RemoveGameplayTag` (`self.EditableItem`) (struct :`TagName` "InteriorItem.Editing.Moving"))
        (message `/Game/Blueprints/Interior/BI_InteriorActorInterface.AddGameplayTag` (`self.EditableItem`) (struct :`TagName` "InteriorItem.Editing"))))))

(event `EventInteriorActorCreated`
  (params (InteriorActor :type "Actor Object Reference"))
  (if (`KismetSystemLibrary.DoesImplementInterface` InteriorActor "/Game/Blueprints/Interior/BI_InteriorActorInterface.BI_InteriorActorInterface_C")
    (bind _output_get (set `self.EditableItem` InteriorActor))
    (message `/Game/Blueprints/Interior/BI_InteriorActorInterface.AddGameplayTag` _output_get (struct :`TagName` "InteriorItem.Placing"))
    (else
      (`KismetSystemLibrary.PrintString` "Created actor doesn't implement InteriorActorInterface!"))))

(event `EventPaletteItemSelected`
  (params (ItemData :type "/Game/InteriorData/F_PaletteItemData Structure"))
  (`self.DestroyInteriorActorIfPlacing`)
  (bind _outdata (`/Game/Blueprints/BP_EditorUtilities.PaletteDataToInteriorActorData` ItemData))
  (`self.OnCreateInteriorActor` _outdata)
  (`self.OnEditRoomActorFinished`))

(event `EventEditableItemMove`
  (message `/Game/Blueprints/Interior/BI_InteriorActorInterface.AddGameplayTag` (`self.EditableItem`) (struct :`TagName` "InteriorItem.Editing.Moving")))

(event `EventEditableItemDelete`
  (`self.OnEditRoomActorFinished`)
  (`Actor.K2_DestroyActor` (`self.EditableItem`))
  (set `self.EditableItem` null))

(event `EventItemColorSelected`
  (params (Color :type "LinearColor Structure"))
  (bind _staticmesh (message `/Game/Blueprints/Interior/BI_InteriorActorInterface.As Static Mesh Actor` (`self.EditableItem`)))
  (bind _staticmeshcomponent (`StaticMeshActor.StaticMeshComponent` _staticmesh))
  (bind _returnvalue (`PrimitiveComponent.CreateDynamicMaterialInstance` _staticmeshcomponent 0 (`PrimitiveComponent.GetMaterial` _staticmeshcomponent 0) "None"))
  (`MaterialInstanceDynamic.SetVectorParameterValue` _returnvalue (`self.MaterialParameterBaseColor`) Color)
  (`PrimitiveComponent.SetMaterial` (`StaticMeshActor.StaticMeshComponent` _staticmesh) 0 _returnvalue))

(fn `DestroyInteriorActorIfPlacing`
  (returns (ActorDestroyed :type Boolean))
  (bind _tags (message `/Game/Blueprints/Interior/BI_InteriorActorInterface.GetGameplayTags` (`self.EditableItem`)))
  (if (`BlueprintGameplayTagLibrary.HasTag` _tags (struct :`TagName` "InteriorItem.Placing") true)
    (`Actor.K2_DestroyActor` (`self.EditableItem`))
    (return true)
    (else
      (return false))))