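; Player pawn that places the selected inventory item in the world at the mouse cursor.
; IA_Select deprojects the cursor into a short line trace against WorldStatic objects and spawns the InventoryComponent's selected class where it hits a floor-tagged actor.
; Two debug keys select the first or second inventory slot.
; IA_ZoomCamera is a placeholder that adds zero-direction movement input, and trace drawing and spawn printing remain for debugging.
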(event Input|EnhancedActionEvents|EnhancedInputActionIA_Select
  (params (ActionValue :type Boolean) (ElapsedSeconds :type Float%20%28double-precision%29) (TriggeredSeconds :type Float%20%28double-precision%29) (InputAction :type Input%20Action%20Object%20Reference :default "/Game/Input/IA_Select.IA_Select"))
  (bind _returnvalue (Pawn|GetLocalViewingPlayerController))
  (bind (_worldlocation _worlddirection) (Game|Player|ConvertMouseLocationToWorldSpace _returnvalue))
  (Class|WidgetLayoutLibrary|GetMousePositiononViewport)
  (bind (_outhit _returnvalue_2) (Collision|LineTraceForObjects _worldlocation (+ _worldlocation (* _worlddirection 1e+03)) (Utilities|Array|MakeArray "ObjectTypeQuery1") false 0 "ForDuration"))
  (if _returnvalue_2
    (if (Actor|ActorHasTag (.HitActor (Collision|BreakHitResult _outhit)) (Variables|Default|GetTagFloor))
      (bind _newparam (Default|GetSelectedItem (Variables|Default|GetInventoryComponent)))
      (bind _returnvalue_3 (Game|SpawnActorfromClass _newparam (Math|Transform|MakeTransform (.Location (Collision|BreakHitResult _outhit))) "AdjustIfPossibleButAlwaysSpawn" "MultiplyWithRoot" self 0))
      (Development|PrintString (Utilities|String|BuildString(Object) "Spawned actor: " "" _returnvalue_3)))))

(event Input|EnhancedActionEvents|EnhancedInputActionIA_ZoomCamera
  (params (ActionValue :type Float%20%28double-precision%29) (ElapsedSeconds :type Float%20%28double-precision%29) (TriggeredSeconds :type Float%20%28double-precision%29) (InputAction :type Input%20Action%20Object%20Reference :default "/Game/Input/IA_ZoomCamera.IA_ZoomCamera"))
  (Pawn|Input|AddMovementInput "0, 0, 0" 1.0 false))

(event EventBeginPlay)

(event Collision|EventActorBeginOverlap
  (params (OtherActor :type Actor%20Object%20Reference)))

(event EventTick
  (params (DeltaSeconds :type Float%20%28single-precision%29)))

(event Input|KeyboardEvents|DebugKey1
  (params (Key :type Key%20Structure :default "None") (ActionValue :type Input%20Action%20Value%20Structure))
  (:Pressed
    (Default|SelectItematPosition (Variables|Default|GetInventoryComponent))))

(event Input|KeyboardEvents|DebugKey2
  (params (Key :type Key%20Structure :default "None") (ActionValue :type Input%20Action%20Value%20Structure))
  (:Pressed
    (Default|SelectItematPosition (Variables|Default|GetInventoryComponent) 1)))

(fn ConstructionScript)